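; BP_Bullet is a projectile actor that flies straight along its forward vector and explodes on contact.
; Tick moves it by Speed scaled by delta time, using a swept SetActorLocation rather than a movement component.
; When its sphere collision begins an overlap, it spawns the P_Explosion emitter at the sweep impact point and destroys itself.
; The graph applies no damage to whatever it overlaps.
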(event OnComponentBeginOverlap(SphereCollision)
  (params (OverlappedComponent :type Primitive%20Component%20Object%20Reference) (OtherActor :type Actor%20Object%20Reference) (OtherComp :type Primitive%20Component%20Object%20Reference) (OtherBodyIndex :type Integer) (bFromSweep :type Boolean) (SweepResult :type Hit%20Result%20Structure%20%28by%20ref%29))
  (Effects|SpawnEmitteratLocation "/Game/StarterContent/Particles/P_Explosion.P_Explosion" (.ImpactPoint (Collision|BreakHitResult SweepResult)))
  (Actor|DestroyActor))

(event EventBeginPlay)

(event Collision|EventActorBeginOverlap
  (params (OtherActor :type Actor%20Object%20Reference)))

(event EventTick
  (params (DeltaSeconds :type Float%20%28single-precision%29))
  (Transformation|SetActorLocation (+ (Transformation|GetActorLocation) (* (* (Transformation|GetActorForwardVector) (Variables|Default|GetSpeed)) DeltaSeconds)) true false))

(fn ConstructionScript)