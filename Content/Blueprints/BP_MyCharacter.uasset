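; Player character Blueprint that provides movement, look and jump through Enhanced Input, registering its mapping context on BeginPlay.
; Move and rotate actions only cache their values on Triggered and Completed, while jump starts and stops directly.
; Tick applies the cached values, moving relative to control rotation, sending yaw to the controller, and pitching the SpringArm directly within a clamped range.
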(event Input|EnhancedActionEvents|EnhancedInputActionIA_Jump_DIP
  (params (ActionValue :type Boolean) (ElapsedSeconds :type Float%20%28double-precision%29) (TriggeredSeconds :type Float%20%28double-precision%29) (InputAction :type Input%20Action%20Object%20Reference :default "/Game/Input/IA_Jump_DIP.IA_Jump_DIP"))
  ;[1 1 1] Input 이벤트 설정하기
  (:Started
    (Character|Jump))
  (:Completed
    (Character|StopJumping)))

(event Input|EnhancedActionEvents|EnhancedInputActionIA_Roate_DIP
  (params (ActionValue :type Vector%202D%20Structure) (ElapsedSeconds :type Float%20%28double-precision%29) (TriggeredSeconds :type Float%20%28double-precision%29) (InputAction :type Input%20Action%20Object%20Reference :default "/Game/Input/IA_Roate_DIP.IA_Roate_DIP"))
  ;[1 1 1] Input 이벤트 설정하기
  (:Triggered
    (Variables|Default|SetRotateAxis (Math|Rotator|MakeRotator 0.0 (.y ActionValue) (.x ActionValue))))
  (:Completed
    (Variables|Default|SetRotateAxis (Math|Rotator|MakeRotator 0.0 (.y ActionValue) (.x ActionValue)))))

(event Input|EnhancedActionEvents|EnhancedInputActionIA_Move_DIP
  (params (ActionValue :type Vector%202D%20Structure) (ElapsedSeconds :type Float%20%28double-precision%29) (TriggeredSeconds :type Float%20%28double-precision%29) (InputAction :type Input%20Action%20Object%20Reference :default "/Game/Input/IA_Move_DIP.IA_Move_DIP"))
  ;[1 1 1] Input 이벤트 설정하기
  (:Triggered
    (Variables|Default|SetMoveDir (Math|Vector|MakeVector (.x ActionValue) (.y ActionValue) 0.0)))
  (:Completed
    (Variables|Default|SetMoveDir (Math|Vector|MakeVector (.x ActionValue) (.y ActionValue) 0.0))))

(event EventBeginPlay
  (bind _asplayer_controller (Utilities|Casting|CastToPlayerController (Pawn|GetController)))
  (Variables|Default|SetPC _asplayer_controller)
  (Input|AddMappingContext (PlayerController|LocalPlayerSubsystems|GetEnhancedInputLocalPlayerSubsystem _asplayer_controller) "/Game/Input/IMC_DIPInput.IMC_DIPInput" 0 "(bIgnoreAllPressedKeysUntilRelease=True,bForceImmediately=False,bNotifyUserSettings=False)"))

(event Collision|EventActorBeginOverlap
  (params (OtherActor :type Actor%20Object%20Reference)))

(event EventTick
  (params (DeltaSeconds :type Float%20%28single-precision%29))
  (bind _movedir (Variables|Default|GetMoveDir))
  (bind _rotateaxis (Variables|Default|GetRotateAxis))
  (bind _springarm (Variables|Default|GetSpringArm))
  (bind _pc (Variables|Default|GetPC))
  (bind _returnvalue (Transformation|GetWorldRotation _springarm))
  (bind _returnvalue_2 (Pawn|GetControlRotation _pc :!class /Script/Engine.Controller))
  (Utilities|IsValid _pc
    (:Is%20Valid
      (Pawn|Input|AddMovementInput (+ (* (Math|Vector|GetForwardVector _returnvalue_2) (.x _movedir)) (* (Math|Vector|GetRightVector _returnvalue_2) (.y _movedir))) 1.0 false)
      (Pawn|Input|AddControllerYawInput (.yaw _rotateaxis))
      (Transformation|SetWorldRotation _springarm (Math|Rotator|MakeRotator (.roll _returnvalue) (Math|Float|Clamp(Float) (+ (.pitch _returnvalue) (.pitch _rotateaxis)) -6e+01 6e+01) (.yaw _returnvalue)) false false))))

(fn ConstructionScript)